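; Game mode for the Futebas football game that hands pre-existing pawns to player controllers.
; On each possess request the controller takes the next PawnArray entry; when two players are in, both pawns receive player and skill settings from Team1 and Team2 in the game instance.
; The older player-versus-bot match flow (goals, restarts, halves, stoppage time) remains as empty events, disconnected logic and leftover "old" functions, as does the code that filled PawnArray.
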(event Custom|antesDoComeco_old
  ;[1 1 1] Antes do Começo
)

(event Custom|golDirBeginOverlap_old
  ;[1 1 1] Gol do time esquerdo
)

(event Custom|golEsqBeginOverlap_old
  ;[1 1 1] Gol do time direito
)

(event Custom|terminaTempo_old
  ;[1 1 1] Termina Tempo
)

(event Custom|reinicia_old
  (params (neutro :type Boolean) (favoravelTimeEsq :type Boolean))
  ;[1 1 1] Restart Game
)

(event Custom|PossessRequested_o
  (params (PC :type Player%20Controller%20Object%20Reference))
  (bind _pawnarray (Variables|Default|GetpawnArray))
  (bind _players (Variables|Default|Getplayers))
  (Development|PrintString "Possess" true true "(R=0.000000,G=1.000000,B=0.074790,A=1.000000)" 2e+01)
  (if (< _players (Utilities|Array|Length _pawnarray))
    (Pawn|Possess PC (Utilities|Array|Get(acopy) _pawnarray _players))
    (bind _result (Math|Integer|IncrementInt (Variables|Default|Getplayers))
      (:%20%20
        (if (== _result 2)
          (bind _asfutebas_game_instance (Utilities|Casting|CastToFutebasGameInstance (Game|GetGameInstance)))
          (for (_array_element _array_index) (Variables|Default|GetpawnArray)
            (switch int _array_index
              (:0
                (Class|OJogoCharacter|PawnConfig _array_element (.jogador (Utilities|Struct|BreakTeamData (Variables|/Script/OJogo.FutebasGameInstance|Getteam1 _asfutebas_game_instance))) (.habilidades (Utilities|Struct|BreakTeamData (Variables|/Script/OJogo.FutebasGameInstance|Getteam1 _asfutebas_game_instance)))))
              (:1
                (Class|OJogoCharacter|PawnConfig _array_element (.jogador (Utilities|Struct|BreakTeamData (Variables|/Script/OJogo.FutebasGameInstance|Getteam2 _asfutebas_game_instance))) (.habilidades (Utilities|Struct|BreakTeamData (Variables|/Script/OJogo.FutebasGameInstance|Getteam2 _asfutebas_game_instance))))))))))))

(event Custom|Escanteio_old
  (params (pos :type Actor%20Object%20Reference))
  ;[1 1 1] Escanteio
)

(event Custom|fimDePapo_old
  ;[1 1 1] Fim de Papo
)

(event Custom|reiniciaBolaMeio_old
  ;[1 1 1] Bola explodida
)

(event EventBeginPlay
  ;[1 1 1] Begin Play
)

(fn ConstructionScript)

(fn MaisAcrescimosOld
  (bind _returnvalue (Utilities|Time|SetTimerbyEvent (EventDispatchers|CreateEvent :!event TerminaTempo) (+ (Math|Conversions|ToFloat(Integer) (Math|Timespan|GetSeconds (Variables|/Game/Levels/JogosGameState_old.JogosGameState_old_C|Getacrescimos (Variables|Default|GetjogosGameState_old)))) 0.1)))
  (Variables|/Game/Levels/JogosGameState_old.JogosGameState_old_C|Settempo2 (Variables|Default|GetjogosGameState_old) _returnvalue)
  (Variables|/Game/Levels/JogosGameState_old.JogosGameState_old_C|SettempoRegulamentar (Variables|Default|GetjogosGameState_old) false))

(fn ComecaJogoOld
  (bind _returnvalue (Utilities|Time|SetTimerbyFunctionName 0 "maisAcrescimos" 45.0))
  (Variables|/Game/Levels/JogosGameState_old.JogosGameState_old_C|Settempo1 (Variables|Default|GetjogosGameState_old) _returnvalue)
  (Variables|/Game/Levels/JogosGameState_old.JogosGameState_old_C|SettempoRegulamentar (Variables|Default|GetjogosGameState_old) true)
  (Variables|/Game/Levels/JogosGameState_old.JogosGameState_old_C|SetbolaEmJogo (Variables|Default|GetjogosGameState_old) true))

(fn TrocaTimesOld
  (bind _futebasgi_old (Variables|Default|GetFutebasGI_old))
  (LocalVariables|Setaux (Variables|/Game/Levels/JogosGameState_old.JogosGameState_old_C|GetgolsTimeEsq (Variables|Default|GetjogosGameState_old)))
  (Variables|/Game/Levels/JogosGameState_old.JogosGameState_old_C|SetgolsTimeEsq (Variables|Default|GetjogosGameState_old) (Variables|/Game/Levels/JogosGameState_old.JogosGameState_old_C|GetgolsTimeDir (Variables|Default|GetjogosGameState_old)))
  (Variables|/Game/Levels/JogosGameState_old.JogosGameState_old_C|SetgolsTimeDir (Variables|Default|GetjogosGameState_old) (LocalVariables|Getaux))
  (LocalVariables|SetteamAux (Variables|/Script/OJogo.FutebasGameInstance|Getteam1 (Variables|Default|GetFutebasGI_old)))
  (Variables|/Script/OJogo.FutebasGameInstance|Setteam1 _futebasgi_old (Variables|/Script/OJogo.FutebasGameInstance|Getteam2 _futebasgi_old))
  (Variables|/Script/OJogo.FutebasGameInstance|Setteam2 (Variables|Default|GetFutebasGI_old) (LocalVariables|GetteamAux))
  (return))

(fn SetBotGolsOld
  (params (golsEsq :type Integer) (golsDir :type Integer)))