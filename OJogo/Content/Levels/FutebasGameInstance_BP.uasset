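; Game instance for the Futebas game that hosts and joins online matches through session nodes.
; HostServer creates a two-player session tagged with stadium, team and room name properties, then opens the stadium level as a listen server.
; JoinServer joins a given search result.
; Both report through on-screen messages in Portuguese, though hosting only prints on failure.
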(event Custom|HostServer
  (params (Stadium :type Name) (team :type String) (roomName :type String))
  (bind _structout (Utilities|Struct|SetmembersinSessionPropertyKeyPair (Class|AdvancedSessionsLibrary|MakeLiteralSessionPropertyString "stadium" (Utilities|String|ToString(Name) Stadium))))
  (bind _structout_2 (Utilities|Struct|SetmembersinSessionPropertyKeyPair (Class|AdvancedSessionsLibrary|MakeLiteralSessionPropertyString "team" team)))
  (bind _structout_3 (Utilities|Struct|SetmembersinSessionPropertyKeyPair (Class|AdvancedSessionsLibrary|MakeLiteralSessionPropertyString "name" roomName)))
  (|AdvancedSession (Utilities|Array|MakeArray _structout _structout_2 _structout_3) (Game|GetPlayerController 0) 2 0 false true false true true false false false true
    (:OnSuccess
      (Game|OpenLevel(byName) Stadium false "?listen"))
    (:OnFailure
      (Development|PrintString "Não foi possível criar a partida" true true "(R=1.000000,G=0.000000,B=0.081863,A=1.000000)" 5.0))))

(event Custom|JoinServer
  (params (SR :type Blueprint%20Session%20Result%20Structure))
  (|JoinSession (Game|GetPlayerController 0) SR
    (:OnSuccess
      (Development|PrintString "Entrando" true true "(R=0.229352,G=1.000000,B=0.000000,A=1.000000)" 5.0))
    (:OnFailure
      (Development|PrintString "Falha ao entrar na partida" true true "(R=1.000000,G=0.000000,B=0.081863,A=1.000000)" 5.0))))