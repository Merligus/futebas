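; Player controller that relays possession requests to the game mode and switches the view to level cameras.
; RPC_PossessRequest_o passes itself to PossessRequest_o, which calls PossessRequestedO on JogosGameMode_BP.
; SetCamera_o blends the view target to every CameraActor that has any tag, so the last one found wins.
; Unconnected leftover nodes reference MultiplayerGM and a Player1_BP Config call.
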(event Custom|PossessRequest_o
  (params (PC :type Player%20Controller%20Object%20Reference))
  (bind _asjogos_game_mode_bp (Utilities|Casting|CastToJogosGameMode_BP (Game|GetGameMode)))
  (Default|PossessRequestedO _asjogos_game_mode_bp PC))

(event Custom|RPC_PossessRequest_o
  (Development|PrintString "PossessRequest" true true "(R=0.561921,G=1.000000,B=0.000000,A=1.000000)" 2e+01)
  (CallFunction|PossessRequestO self))

(event Custom|SetCamera_o
  (bind _outactors (Actor|GetAllActorsOfClass "/Script/Engine.CameraActor"))
  (for _array_element _outactors
    (if (> (Utilities|Array|Length (Variables|/Script/Engine.Actor|GetTags _array_element)) 0)
      (Development|PrintString "Camera" true true "(R=0.997933,G=1.000000,B=0.000000,A=1.000000)" 2e+01)
      (Game|Player|SetViewTargetwithBlend self _array_element 0.0 "VTBlend_Linear" 0.0 true))))

(event EventBeginPlay)

(event EventPossess
  (params (PossessedPawn :type Pawn%20Object%20Reference)))

(fn ConstructionScript)